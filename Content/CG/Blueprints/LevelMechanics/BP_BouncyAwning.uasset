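; BP_BouncyAwning is a level mechanic that bounces the player when they touch the awning's collider.
; It caches the first player character on BeginPlay and checks each Collider overlap against that player's pawn.
; On a match it adds BounceHeight to the character movement as a velocity-change impulse, ignoring mass, and prints a debug "Hello".
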(event `self.ReceiveBeginPlay`
  (set `self.PlayerRef` (`GameplayStatics.GetPlayerCharacter` 0)))

(event `self.Collider.OnComponentBeginOverlap`
  (params (OverlappedComponent :type "PrimitiveComponent Object Reference") (OtherActor :type "Actor Object Reference") (OtherComp :type "PrimitiveComponent Object Reference") (OtherBodyIndex :type Integer) (bFromSweep :type Boolean) (SweepResult :type "HitResult Structure (by ref)"))
  (if (== OtherActor (`GameplayStatics.GetPlayerPawn` 0))
    (`CharacterMovementComponent.AddImpulse` (`Character.CharacterMovement` (`self.PlayerRef`)) (`self.BounceHeight`) true)
    (`KismetSystemLibrary.PrintString` "Hello")))

(fn `UserConstructionScript`)