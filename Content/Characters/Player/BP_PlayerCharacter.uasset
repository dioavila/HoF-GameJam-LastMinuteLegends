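; BP_PlayerCharacter is the player character Blueprint, providing knockback and launch reactions through custom events.
; BeginPlay stores the world transform of the CameraPlayer component in CameraTransform.
; PlayerKnockback and PlayerLaunch apply velocity-change impulses scaled from current movement velocity, one reversed and amplified, the other amplifying the vertical component.
; Both impulses therefore depend on existing motion and add nothing when the character is stationary.
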(event `self.ReceiveBeginPlay`
  (set `self.CameraTransform` (`SceneComponent.K2_GetComponentToWorld` (`self.cameraPlayer`))))

(event `PlayerKnockback`
  (bind _charactermovement (`self.CharacterMovement`))
  (`CharacterMovementComponent.AddImpulse` _charactermovement (* (`MovementComponent.Velocity` _charactermovement) (-5.0 -5.0 -5.0)) true))

(event `PlayerLaunch`
  (bind _charactermovement (`self.CharacterMovement`))
  (`CharacterMovementComponent.AddImpulse` _charactermovement (* (`MovementComponent.Velocity` _charactermovement) (1.0 1.0 5.0)) true))

(fn `UserConstructionScript`)